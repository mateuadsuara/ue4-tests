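; BP_Spinning_Logo is a Blueprint communication prop whose logo starts or stops spinning each time its PushedButton event fires.
; A FlipFlop alternates between swapping the logo material while playing a looping Rotation timeline that drives relative yaw, and switching the material while turning looping off.
; Stopping only clears the loop flag, so the current turn finishes rather than halting abruptly.
; The GrabInteract interface function is a stub returning zeros.
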(event EventPushedButton
  (bind _rotation (Variables|Default|GetRotation))
  (bind _logo (Variables|BP_Spinning_Logo|GetLogo))
  ;[1 1 1] Toggle the spinning animation
  (Utilities|FlowControl|FlipFlop
    (:A
      (Rendering|Material|SetMaterial _logo 0 "/Game/DemoRoom/Materials/M_UE4_Logo_Doors.M_UE4_Logo_Doors")
      (Components|Timeline|SetLooping _rotation true)
      (bind _yaw_value (Timeline|Rotation Play)
        (:Update
          (Transformation|SetRelativeRotation (Variables|BP_Spinning_Logo|GetLogo) (Class|KismetMathLibrary|MakeRot 0.0 _yaw_value 0.0) false))))
    (:B
      (Rendering|Material|SetMaterial _logo 0 "/Game/DemoRoom/Materials/M_UE4_Logo_Door.M_UE4_Logo_Door")
      (Components|Timeline|SetLooping _rotation false))))

(fn ConstructionScript)

(fn GrabInteract
  (params (Player%20aim%20movement :type Vector%202D%20Structure) (Interacting :type Boolean))
  ;[1 1 1] Interface for Grab Interaction
  (return ""))