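; BP_ButtonLight_Bulb_Basic is a button prop from a Blueprint communication folder that switches a target light through a trigger collision.
; Begin and end overlap share one FlipFlop, so every overlap event alternates between on and off.
; Each flip sets the State parameter on the button's dynamic material, created in the construction script, and calls ToggleLight on TargetLight to match.
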(event OnComponentBeginOverlap(Triggercollision)
  (params (OtherActor :type Actor%20Object%20Reference) (OtherComp :type Primitive%20Component%20Object%20Reference) (OtherBodyIndex :type Integer))
  (bind _button_light_material (Variables|Default|GetButton%20light%20material))
  (bind _target_light (Variables|Default|GetTarget%20light))
  (Utilities|FlowControl|FlipFlop
    (:A
      (Rendering|Material|SetScalarParameterValue _button_light_material "State" 1.0 :!class /Script/Engine.MaterialInstanceDynamic)
      (Default|ToggleLight _target_light true))
    (:B
      (Rendering|Material|SetScalarParameterValue _button_light_material "State" 0.0 :!class /Script/Engine.MaterialInstanceDynamic)
      (Default|ToggleLight _target_light false))))

(event OnComponentEndOverlap(Triggercollision)
  (params (OtherActor :type Actor%20Object%20Reference) (OtherComp :type Primitive%20Component%20Object%20Reference) (OtherBodyIndex :type Integer))
  (bind _button_light_material (Variables|Default|GetButton%20light%20material))
  (bind _target_light (Variables|Default|GetTarget%20light))
  (Utilities|FlowControl|FlipFlop
    (:A
      (Rendering|Material|SetScalarParameterValue _button_light_material "State" 1.0 :!class /Script/Engine.MaterialInstanceDynamic)
      (Default|ToggleLight _target_light true))
    (:B
      (Rendering|Material|SetScalarParameterValue _button_light_material "State" 0.0 :!class /Script/Engine.MaterialInstanceDynamic)
      (Default|ToggleLight _target_light false))))

(fn ConstructionScript
  (bind _returnvalue (Rendering|Material|CreateDynamicMaterialInstance (Variables|Default|GetButtonMesh) 2 0 :!class /Script/Engine.PrimitiveComponent))
  (Variables|Default|SetButton%20light%20material _returnvalue))