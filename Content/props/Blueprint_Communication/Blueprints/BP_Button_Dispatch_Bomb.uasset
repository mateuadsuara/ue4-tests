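; BP_Button_Dispatch_Bomb is an overlap-triggered button that spawns a BP_Bomb at an offset from itself.
; On activation it disables itself, switches its light through a dynamic material parameter and binds to the bomb's BombExploded dispatcher.
; After the explosion callback it waits briefly, resets the light and re-enables, then fires again if something still overlaps the trigger.
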(event OnComponentBeginOverlap(Triggercollision)
  (params (OtherActor :type Actor%20Object%20Reference) (OtherComp :type Primitive%20Component%20Object%20Reference) (OtherBodyIndex :type Integer))
  (Variables|Default|SetOverlapping%20button true)
  (if (Variables|Default|GetButton%20enabled)
    (CallFunction|Activate)))

(event OnComponentEndOverlap(Triggercollision)
  (params (OtherActor :type Actor%20Object%20Reference) (OtherComp :type Primitive%20Component%20Object%20Reference) (OtherBodyIndex :type Integer))
  (Variables|Default|SetOverlapping%20button false))

(event Custom|Activate
  (Variables|Default|SetButton%20enabled false)
  (Rendering|Material|SetScalarParameterValue (Variables|Default|GetButton%20light%20material) "State" 1.0 :!class /Script/Engine.MaterialInstanceDynamic)
  (bind _returnvalue (Game|SpawnActorfromClass "/Game/ExampleContent/Blueprint_Communication/Blueprints/BP_Bomb.BP_Bomb_C" (Math|Conversions|ToTransform(Vector) (+ (Transformation|GetActorLocation) (Variables|Default|GetSpawn%20point))) true))
  (EventDispatchers|BindEventtoBombExploded _returnvalue (delegate Custom|Bomb%20Exploded_Event)))

(event Custom|Bomb%20Exploded_Event
  (Utilities|FlowControl|Delay 1.0)
  (Rendering|Material|SetScalarParameterValue (Variables|Default|GetButton%20light%20material) "State" 0.0 :!class /Script/Engine.MaterialInstanceDynamic)
  (Variables|Default|SetButton%20enabled true)
  (Utilities|FlowControl|Delay 0.1)
  (if (Variables|Default|GetOverlapping%20button)
    (CallFunction|Activate)))

(fn ConstructionScript
  (bind _returnvalue (Rendering|Material|CreateDynamicMaterialInstance (Variables|Default|GetButtonMesh) 2 0 :!class /Script/Engine.PrimitiveComponent))
  (Variables|Default|SetButton%20light%20material _returnvalue))